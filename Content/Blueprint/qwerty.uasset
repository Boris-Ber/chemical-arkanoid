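; Block-grid actor for a recipe-matching puzzle that spawns a row of random-material cubes every four seconds, pushing older rows along Y.
; Each cube gets a material-name label and particle component, indexed in maps by name and sequential ID.
; ne_stukai checks a given texture against the target block's Recepies row.
; A match triggers Chainreaction, a recursive flood fill using nine-wide ID arithmetic to destroy adjacent same-material blocks.
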(event Custom|ne_stukai
  (params (bonk :type String) (texture :type Material%20Interface%20Object%20Reference))
  (bind _blocks (Variables|Default|Getblocks))
  (bind _value (Utilities|Map|Find _blocks bonk))
  (bind _returnvalue (Rendering|Material|GetMaterial _value 0))
  (bind _returnvalue_2 (Utilities|GetDataTableRow (Variables|Default|Getrecepies) (.Value (Utilities|Map|Find (Variables|Default|Getmaterial-name) _returnvalue)))
    (:then
      (bind _result (Utilities|Set|ToArray (Utilities|Set|MakeSet (.1 (Utilities|Struct|Breakcombos _returnvalue_2)) (.2 (Utilities|Struct|Breakcombos _returnvalue_2)) (.3 (Utilities|Struct|Breakcombos _returnvalue_2)) (.4 (Utilities|Struct|Breakcombos _returnvalue_2)) (.5 (Utilities|Struct|Breakcombos _returnvalue_2)) (.6 (Utilities|Struct|Breakcombos _returnvalue_2)) (.7 (Utilities|Struct|Breakcombos _returnvalue_2)) (.8 (Utilities|Struct|Breakcombos _returnvalue_2)) (.9 (Utilities|Struct|Breakcombos _returnvalue_2)) (.10 (Utilities|Struct|Breakcombos _returnvalue_2)) (.11 (Utilities|Struct|Breakcombos _returnvalue_2)) (.12 (Utilities|Struct|Breakcombos _returnvalue_2)) (.13 (Utilities|Struct|Breakcombos _returnvalue_2)))))
      (if (!= (Utilities|Array|FindItem _result texture) -1)
        (CallFunction|Chain-reaction bonk _returnvalue)))))

(event EventBeginPlay
  (bind _blocks (Variables|Default|Getblocks))
  (bind _index (Variables|Default|Getindex))
  (bind _keys (Utilities|Map|Keys _blocks :!label _label))
  (for _array_element _keys
    (Transformation|AddWorldOffset (.Value (Utilities|Map|Find _blocks _array_element)) (Math|Vector|MakeVector 0.0 2.2e+02 0.0) false false))
  (Variables|Default|Settochka "0, 0, 0")
  (for _index_2 (range 0 8)
    (bind _returnvalue (AddComponent|AddStaticMeshComponent false (Math|Transform|MakeTransform (Variables|Default|Gettochka) "0, 0, 0" "2.000000,2.000000,2.000000")))
    (Rendering|Material|SetMaterial _returnvalue 0 (.OutItem (Utilities|Array|Random (Variables|Default|GetElem_cube))))
    (bind _returnvalue_2 (AddComponent|AddParticleSystemComponent false (Math|Transform|MakeTransform (Variables|Default|Gettochka) "0, 0, 0" "5.000000,5.000000,5.000000")))
    (Transformation|AttachComponentToComponent _returnvalue_2 _returnvalue "None" "KeepWorld" "KeepWorld" "KeepWorld" false)
    (bind _returnvalue_3 (AddComponent|AddTextRenderComponent false (Math|Transform|MakeTransform (Math|Vector|MakeVector (- (.x (Variables|Default|Gettochka)) 5e+01) (- (.y (Variables|Default|Gettochka)) -1e+02) (+ (.z (Variables|Default|Gettochka)) 205.0)) "90.000000,90.000000,0.000000" "6.500000,6.500000,6.500000")))
    (Rendering|Components|TextRender|SetText _returnvalue_3 (Utilities|Text|ToText(Name) (.Value (Utilities|Map|Find (Variables|Default|Getmaterial-name) (Rendering|Material|GetMaterial _returnvalue 0)))))
    (Transformation|AttachComponentToComponent _returnvalue_3 _returnvalue "None" "KeepWorld" "KeepWorld" "KeepWorld" true)
    (Variables|Default|Settochka (Math|Vector|MakeVector (+ (.x (Variables|Default|Gettochka)) 2.2e+02) 0.0 0.0))
    (Utilities|Map|Add (Variables|Default|Getblocks) (Utilities|GetDisplayName _returnvalue) _returnvalue)
    (Utilities|Map|Add (Variables|Default|Getcube-id) (Utilities|GetDisplayName _returnvalue) _index)
    (Utilities|Map|Add (Variables|Default|Getid-cube) _index (Utilities|GetDisplayName _returnvalue))
    (Math|Integer|IncrementInt _index
      (:%20%20
        (Utilities|Map|Add (Variables|Default|Gettext) (Utilities|GetDisplayName _returnvalue) _returnvalue_3)
        (Utilities|Map|Add (Variables|Default|Getboom) (Utilities|GetDisplayName _returnvalue) _returnvalue_2))))
  (Utilities|FlowControl|Delay 4.0)
  (goto _label))

(event Collision|EventActorBeginOverlap
  (params (OtherActor :type Actor%20Object%20Reference)))

(event EventTick
  (params (DeltaSeconds :type Float%20%28single-precision%29)))

(fn ConstructionScript)

(fn Chain-reaction
  (params (name :type String) (cube-color :type Material%20Interface%20Object%20Reference))
  (bind _cube_id (Variables|Default|Getcube-id))
  (bind _id_cube (Variables|Default|Getid-cube))
  (bind _text (Variables|Default|Gettext))
  (bind _boom (Variables|Default|Getboom))
  (bind _blocks (Variables|Default|Getblocks))
  (bind _value (Utilities|Map|Find _cube_id name))
  (bind (_value_2 _returnvalue) (Utilities|Map|Find _blocks name))
  (bind _returnvalue_2 (- _value 9))
  (bind _returnvalue_3 (+ _value 9))
  (bind (_value_3 _returnvalue_4) (Utilities|Map|Find _id_cube _returnvalue_3))
  (bind (_value_4 _returnvalue_5) (Utilities|Map|Find _id_cube _returnvalue_2))
  (if _returnvalue
    (if (== cube-color (Rendering|Material|GetMaterial _value_2 0))
      (Components|DestroyComponent _value_2)
      (Components|DestroyComponent (.Value (Utilities|Map|Find _text name)))
      (Components|DestroyComponent (.Value (Utilities|Map|Find _boom name)))
      (Utilities|Map|Remove _blocks name)
      (Utilities|Map|Remove _boom name)
      (Utilities|Map|Remove _text name)
      (Utilities|FlowControl|Sequence
        (:then_0
          (switch int (Math|Integer|%(Integer) _value 9)
            (:Default
              (Utilities|FlowControl|Sequence
                (:then_0
                  (CallFunction|Chain-reaction (.Value (Utilities|Map|Find _id_cube (+ _value 1))) cube-color :!label _label))
                (:then_1
                  (CallFunction|Chain-reaction (.Value (Utilities|Map|Find _id_cube (- _value 1))) cube-color :!label _label_2))))
            (:0
              (goto _label_2))
            (:1
              (goto _label))))
        (:then_1
          (Utilities|FlowControl|Sequence
            (:then_0
              (if _returnvalue_5
                (CallFunction|Chain-reaction _value_4 cube-color)))
            (:then_1
              (if _returnvalue_4
                (CallFunction|Chain-reaction _value_3 cube-color)))))))))