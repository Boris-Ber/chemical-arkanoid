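; Launcher actor with a cube and an aim arrow that the player steers before a one-time launch.
; BeginPlay adds the test Enhanced Input mapping context to the player's CustomController.
; Left and right inputs step the arrow's yaw within a clamped arc while it is visible.
; Launch calls the Launch dispatcher once, then hides cube and arrow and disables the cube's collision.
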(event Input|EnhancedActionEvents|EnhancedInputActionLaunch
  (params (ActionValue :type Boolean) (ElapsedSeconds :type Float%20%28double-precision%29) (TriggeredSeconds :type Float%20%28double-precision%29) (InputAction :type Input%20Action%20Object%20Reference :default "/Game/Blueprint/Launch.Launch"))
  (bind _cube (Variables|Default|GetCube))
  (:Started
    (if (not (Variables|Default|GetLaunched))
      (Variables|Default|SetLaunched true)
      (Default|CallLaunch)
      (Rendering|SetVisibility _cube false false)
      (Rendering|SetVisibility (Variables|Default|GetArrow) false false)
      (Collision|SetCollisionEnabled _cube "NoCollision"))))

(event Input|EnhancedActionEvents|EnhancedInputActionMoveLeft
  (params (ActionValue :type Boolean) (ElapsedSeconds :type Float%20%28double-precision%29) (TriggeredSeconds :type Float%20%28double-precision%29) (InputAction :type Input%20Action%20Object%20Reference :default "/Game/Blueprint/MoveLeft.MoveLeft"))
  (if (Rendering|IsVisible (Variables|Default|GetArrow))
    (if (> (Variables|Default|GetDelta) -175.0)
      (Variables|Default|SetDelta (- (Variables|Default|GetDelta) 5.0))
      (Transformation|SetWorldRotation (Variables|Default|GetArrow) (Math|Rotator|MakeRotator 0.0 0.0 (Variables|Default|GetDelta)) false false))))

(event Input|EnhancedActionEvents|EnhancedInputActionMoveRight
  (params (ActionValue :type Boolean) (ElapsedSeconds :type Float%20%28double-precision%29) (TriggeredSeconds :type Float%20%28double-precision%29) (InputAction :type Input%20Action%20Object%20Reference :default "/Game/Blueprint/MoveRight.MoveRight"))
  (if (Rendering|IsVisible (Variables|Default|GetArrow))
    (if (< (Variables|Default|GetDelta) 5.0)
      (Variables|Default|SetDelta (+ (Variables|Default|GetDelta) 5.0))
      (Transformation|SetWorldRotation (Variables|Default|GetArrow) (Math|Rotator|MakeRotator 0.0 0.0 (Variables|Default|GetDelta)) false false))))

(event EventBeginPlay
  (bind _ascustom_controller (Utilities|Casting|CastToCustomController (Game|GetPlayerController 0)))
  (Input|AddMappingContext (PlayerController|LocalPlayerSubsystems|GetEnhancedInputLocalPlayerSubsystem _ascustom_controller) "/Game/Blueprint/MC_Test.MC_Test" 0 "(bIgnoreAllPressedKeysUntilRelease=True,bForceImmediately=False,bNotifyUserSettings=False)"))

(event Collision|EventActorBeginOverlap
  (params (OtherActor :type Actor%20Object%20Reference)))

(event EventTick
  (params (DeltaSeconds :type Float%20%28single-precision%29)))

(fn ConstructionScript)