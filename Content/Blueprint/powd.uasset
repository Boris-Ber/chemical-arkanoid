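; Actor Blueprint (powd) that creates a burst of randomly scattered mesh pieces, stored as Salt, and flings them along world Y.
; BeginPlay spawns the mesh components with random position around LocationBase, rotation and scale, applies Mat, then starts a looping timer.
; Each Fly tick offsets every piece by Speed, incrementing it per piece, so motion accelerates rapidly.
; On Destroyed, it destroys the pieces and clears the array.
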(event Custom|Fly
  (bind _speed (Variables|Default|Getspeed))
  (for _array_element (Variables|Default|Getsalt)
    (Transformation|AddWorldOffset _array_element (Math|Vector|MakeVector 0.0 _speed 0.0) false false)
    (Math|Float|IncrementFloat _speed)))

(event EventBeginPlay
  (bind _returnvalue (Math|Random|RandomFloatinRange -1.8e+02 1.8e+02))
  (bind _returnvalue_2 (Math|Random|RandomFloatinRange 0.4 0.7))
  (bind _location_base (Variables|Default|Getlocation_base))
  (for _index (range 0 20)
    (bind _returnvalue_3 (AddComponent|AddStaticMeshComponent false (Math|Transform|MakeTransform (Math|Vector|MakeVector (Math|Random|RandomFloatinRange (- (.x _location_base) 1e+02) (+ (.x _location_base) 1e+02)) (Math|Random|RandomFloatinRange (- (.y _location_base) 1e+02) (+ (.y _location_base) 1e+02)) (Math|Random|RandomFloatinRange (- (.z _location_base) 1e+02) (+ (.z _location_base) 1e+02))) (Math|Rotator|MakeRotator _returnvalue _returnvalue _returnvalue) (Math|Vector|MakeVector _returnvalue_2 _returnvalue_2 _returnvalue_2))))
    (Rendering|Material|SetMaterial _returnvalue_3 0 (Variables|Default|GetMat))
    (Utilities|Array|Add (Variables|Default|Getsalt) _returnvalue_3))
  (bind _returnvalue_4 (Utilities|Time|SetTimerbyEvent (delegate Custom|Fly) 0.025 true))
  (Variables|Default|SetFlyTimer _returnvalue_4))

(event Collision|EventActorBeginOverlap
  (params (OtherActor :type Actor%20Object%20Reference)))

(event EventDestroyed
  (bind _salt (Variables|Default|Getsalt))
  (for _array_element _salt
    (Components|DestroyComponent _array_element))
  (Utilities|Array|Clear _salt))

(fn ConstructionScript)