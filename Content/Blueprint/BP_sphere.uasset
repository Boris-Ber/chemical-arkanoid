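; BP_sphere is a ball that launches when the player's Bar pawn signals and scores points by hitting qwerty actors.
; On BeginPlay it binds to the Bar's launch event, then adds force to Sfera using Speed and the tangent of an angle derived from the Bar's Delta.
; Hits on qwerty actors call NeStukai with component name, ball material and itself, then increment the Bar's Score and refresh its HUD counter.
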(event OnComponentHit(sfera)
  (params (HitComponent :type Primitive%20Component%20Object%20Reference) (OtherActor :type Actor%20Object%20Reference) (OtherComp :type Primitive%20Component%20Object%20Reference) (NormalImpulse :type Vector :default "0, 0, 0") (Hit :type Hit%20Result%20Structure%20%28by%20ref%29))
  (bind _asqwerty (Utilities|Casting|CastToqwerty OtherActor))
  (Default|NeStukai _asqwerty (Utilities|GetDisplayName OtherComp) (Rendering|Material|GetMaterial (Variables|Default|Getsfera) 0) self)
  (bind _asbar (Utilities|Casting|CastToBar (Game|Player|GetPlayerPawn 0)))
  (bind _result (Math|Float|IncrementFloat (Variables|/Game/Blueprint/bar.Bar_C|Getscore _asbar))
    (:%20%20
      (Variables|/Game/Blueprint/bar.Bar_C|Setscore _asbar _result)
      (Default|UpdateCounterText (Variables|/Game/Blueprint/bar.Bar_C|GetHUDWidget _asbar)))))

(event Custom|Launch
  (bind _speed (Variables|Default|Getspeed))
  (bind _returnvalue (* _speed -1.0))
  (bind _asbar (Utilities|Casting|CastToBar (Game|Player|GetPlayerPawn 0)))
  (Physics|AddForce (Variables|Default|Getsfera) (Math|Vector|MakeVector (* (Math|Trig|Tan(Degrees) (- -9e+01 (Variables|/Game/Blueprint/bar.Bar_C|GetDelta _asbar))) _returnvalue) _returnvalue 0.0) "None" false))

(event Collision|EventActorBeginOverlap
  (params (OtherActor :type Actor%20Object%20Reference)))

(event EventBeginPlay
  (bind _asbar (Utilities|Casting|CastToBar (Game|Player|GetPlayerPawn 0)))
  (EventDispatchers|BindEventtoLaunch _asbar (delegate Custom|Launch)))

(fn ConstructionScript)