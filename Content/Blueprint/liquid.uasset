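; Liquid actor that produces a flying water-fall effect from static mesh pieces when its water-fall event fires.
; A delayed loop adds up to 15 meshes with random position and scale around a base location, applies a material and stores them in the Salt array.
; A looping timer pushes them along Y, raising the shared Speed after each piece moves, so motion keeps accelerating.
; Destroyed removes the meshes.
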(event Custom|Fly
  (bind _speed (Variables|Default|Getspeed))
  (for _array_element (Variables|Default|Getsalt)
    (Transformation|AddWorldOffset _array_element (Math|Vector|MakeVector 0.0 _speed 0.0) false false)
    (Math|Float|IncrementFloat _speed)))

(event Custom|water-fall
  (bind _returnvalue (Math|Random|RandomFloatinRange 2e+01 5e+01))
  (bind _location_base (Variables|Default|Getlocation_base))
  (Utilities|FlowControl|Sequence
    (:then_0
      (if (< (Variables|Default|Getit) 15) :!label _label
        (bind _returnvalue_2 (AddComponent|AddStaticMeshComponent false (Math|Transform|MakeTransform (Math|Vector|MakeVector (Math|Random|RandomFloatinRange (- (.x _location_base) 1e+02) (+ (.x _location_base) 1e+02)) (Math|Random|RandomFloatinRange (- (.y _location_base) 1e+02) (+ (.y _location_base) 1e+02)) (Math|Random|RandomFloatinRange (- (.z _location_base) 1e+02) (+ (.z _location_base) 1e+02))) "0.000000,0.000000,45.000000" (Math|Vector|MakeVector _returnvalue _returnvalue _returnvalue))))
        (Rendering|Material|SetMaterial _returnvalue_2 0 (Variables|Default|GetMat))
        (Utilities|Array|Add (Variables|Default|Getsalt) _returnvalue_2)
        (Utilities|FlowControl|Delay 0.05)
        (Math|Integer|IncrementInt (Variables|Default|Getit)
          (:%20%20
            (goto _label)))))
    (:then_1
      (bind _returnvalue_3 (Utilities|Time|SetTimerbyEvent (delegate Custom|Fly) 0.025 true))
      (Variables|Default|SetFlyTimer _returnvalue_3))))

(event Collision|EventActorBeginOverlap
  (params (OtherActor :type Actor%20Object%20Reference)))

(event EventDestroyed
  (bind _salt (Variables|Default|Getsalt))
  (for _array_element _salt
    (Components|DestroyComponent _array_element))
  (Utilities|Array|Clear _salt))

(fn ConstructionScript)