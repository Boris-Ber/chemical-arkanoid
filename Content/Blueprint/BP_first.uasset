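; BP_first is an actor whose cube jitters around randomly, then animates its scale and destroys itself.
; From BeginPlay, a delayed loop nudges the cube with swept random XY offsets, incrementing a counter each step.
; Component hits also increment and print the counter through the Add function, shortening the wandering.
; Once the counter passes its threshold, a timeline drives uniform cube scale, followed by a short delay before destruction.
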(event OnComponentHit(Cube)
  (params (HitComponent :type Primitive%20Component%20Object%20Reference) (OtherActor :type Actor%20Object%20Reference) (OtherComp :type Primitive%20Component%20Object%20Reference) (NormalImpulse :type Vector :default "0, 0, 0") (Hit :type Hit%20Result%20Structure%20%28by%20ref%29))
  (bind _newparam (CallFunction|Add (Variables|Default|Getnumber)))
  (bind _output_get (Variables|Default|Setnumber _newparam))
  (Development|PrintString (Utilities|String|ToString(Integer) _output_get)))

(event EventBeginPlay
  (if (> (Variables|Default|Getnumber) 15) :!label _label
    (bind _newtrack_0 (Timeline|Timeline PlayFromStart)
      (:Update
        (Transformation|SetWorldScale3D (Variables|Default|GetCube) (Math|Vector|MakeVector _newtrack_0 _newtrack_0 _newtrack_0)))
      (:Finished
        (Utilities|FlowControl|Delay 0.2)
        (Actor|DestroyActor)))
    (else
      (Utilities|FlowControl|Delay 0.2)
      (Transformation|AddWorldOffset (Variables|Default|GetCube) (Math|Vector|MakeVector (Math|Random|RandomFloatinRange -1e+02 1e+02) (Math|Random|RandomFloatinRange -1e+02 1e+02) 0.0) true false)
      (Math|Integer|IncrementInt (Variables|Default|Getnumber)
        (:%20%20
          (goto _label))))))

(event Collision|EventActorBeginOverlap
  (params (OtherActor :type Actor%20Object%20Reference)))

(event EventTick
  (params (DeltaSeconds :type Float%20%28single-precision%29)))

(fn ConstructionScript)

(fn Add
  (params (number :type Integer))
  (return (+ number 1)))